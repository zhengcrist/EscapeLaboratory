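; Spline-driven wire actor that builds its spline mesh segments in the Construction Script.
; SplineMeshVar selects one segment per spline point pair or segments at fixed Spacing along the length with scaled direction tangents.
; WireVar picks the component variant and material slots; WireSize sets thickness.
; Each segment gets two dynamic MI_Wire instances driven by color, dirt, specular, roughness and a TextureVar texture set.
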(fn ConstructionScript
  (|Wire))