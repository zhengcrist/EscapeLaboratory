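; Automatic sliding double door for the science lab that opens when a BP_Body enters its collision volume and closes when it leaves.
; The DoorsManager timeline slides the two leaves apart in opposite directions, randomly picking one of two opening curves per entry and reversing on exit.
; The construction script applies door materials and selects glass or opaque panels from DoorType.
; Directional sound playback exists but is disconnected.
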(event OnComponentBeginOverlap(Collision)
  (params (OverlappedComponent :type Primitive%20Component%20Object%20Reference) (OtherActor :type Actor%20Object%20Reference) (OtherComp :type Primitive%20Component%20Object%20Reference) (OtherBodyIndex :type Integer) (bFromSweep :type Boolean) (SweepResult :type Hit%20Result%20Structure%20%28by%20ref%29))
  (Utilities|Casting|CastToBP_Body OtherActor)
  (Variables|Default|SetOpeningType (Math|Random|RandomBool))
  (bind (_direction _opening1 _opening2) (Timeline|DoorsManager Play)
    (:Update
      (Transformation|SetRelativeLocation (Variables|Default|GetLabDoor03A) (Math|Vector|MakeVector 0.0 (* (Math|Float|Lerp 0.0 9e+01 (select (Variables|Default|GetOpeningType) _opening2 _opening1)) -1.0) 0.0) false false)
      (Transformation|SetRelativeLocation (Variables|Default|GetLabDoor03B) (Math|Vector|MakeVector 0.0 (Math|Float|Lerp 0.0 9e+01 (select (Variables|Default|GetOpeningType) _opening2 _opening1)) 0.0) false false))
    (:Opening
      (switch Utilities|FlowControl|Switch|SwitchonETimelineDirection _direction))
    (:Closing
      (switch Utilities|FlowControl|Switch|SwitchonETimelineDirection _direction))))

(event OnComponentEndOverlap(Collision)
  (params (OverlappedComponent :type Primitive%20Component%20Object%20Reference) (OtherActor :type Actor%20Object%20Reference) (OtherComp :type Primitive%20Component%20Object%20Reference) (OtherBodyIndex :type Integer))
  (Utilities|Casting|CastToBP_Body OtherActor)
  (bind (_direction _opening1 _opening2) (Timeline|DoorsManager Reverse)
    (:Update
      (Transformation|SetRelativeLocation (Variables|Default|GetLabDoor03A) (Math|Vector|MakeVector 0.0 (* (Math|Float|Lerp 0.0 9e+01 (select (Variables|Default|GetOpeningType) _opening2 _opening1)) -1.0) 0.0) false false)
      (Transformation|SetRelativeLocation (Variables|Default|GetLabDoor03B) (Math|Vector|MakeVector 0.0 (Math|Float|Lerp 0.0 9e+01 (select (Variables|Default|GetOpeningType) _opening2 _opening1)) 0.0) false false))
    (:Opening
      (switch Utilities|FlowControl|Switch|SwitchonETimelineDirection _direction))
    (:Closing
      (switch Utilities|FlowControl|Switch|SwitchonETimelineDirection _direction))))

(fn ConstructionScript
  (bind _labdoor03b (Variables|Default|GetLabDoor03B))
  (bind _labdoorjamb03 (Variables|Default|GetLabDoorjamb03))
  (Rendering|Material|SetMaterial _labdoorjamb03 0 "/Game/ScienceLab/Materials/Rooms/Doors/MI_LabDoors01.MI_LabDoors01")
  (Rendering|Material|SetMaterial _labdoorjamb03 1 "/Game/ScienceLab/Materials/Rooms/Doors/MI_LabDoors01.MI_LabDoors01")
  (switch Utilities|FlowControl|Switch|SwitchonEDoorType (Variables|Default|GetDoorType)
    (:NewEnumerator2
      (Rendering|Material|SetMaterial _labdoor03b 2 "/Game/ScienceLab/Materials/Rooms/Doors/MI_Doors_Glass.MI_Doors_Glass"))
    (:NewEnumerator3
      (Rendering|Material|SetMaterial _labdoor03b 2 "/Game/ScienceLab/Materials/Rooms/Wall/MI_Wall01.MI_Wall01"))))